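; BP_PersonInTheWood is a figure in the woods, apparently meant to move along a spline when the player enters its trigger box.
; The construction script applies the chosen skeletal mesh and the trigger box's location and scale.
; BeginPlay caches the first-person player and snaps the Arrow to the first spline point.
; Player overlap restarts the GoToNextPoint timeline, but no movement is wired to it and the next-point lookup is unused.
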(event `self.ReceiveBeginPlay`
  (bind (_returnvalue_inputkey _returnvalue_position) (break `SplinePoint` (`SplineComponent.GetSplinePointAt` (`self.SplinePath`) 0 "World")))
  (bind _asbp_first_person_character (cast `/Game/FirstPerson/Blueprints/BP_FirstPersonCharacter` (`GameplayStatics.GetPlayerCharacter` 0)))
  (set `self.PlayerRef` _asbp_first_person_character)
  (`SceneComponent.K2_SetWorldLocation` (`self.Arrow`) _returnvalue_position false false)
  (set `self.NextPoint` 1))

(event `self.TriggerBox.OnComponentBeginOverlap`
  (params (OverlappedComponent :type "PrimitiveComponent Object Reference") (OtherActor :type "Actor Object Reference") (OtherComp :type "PrimitiveComponent Object Reference") (OtherBodyIndex :type Integer) (bFromSweep :type Boolean) (SweepResult :type "HitResult Structure (by ref)"))
  (if (== OtherActor (`self.PlayerRef`))
    (`Timeline|GoToNextPoint` :!via `PlayFromStart`)))

(fn `UserConstructionScript`
  (bind _triggerbox (`self.TriggerBox`))
  (`SkeletalMeshComponent.SetSkeletalMeshAsset` (`self.MovingEntity`) (`self.MeshDisplayed`))
  (`SceneComponent.K2_SetRelativeLocation` _triggerbox (`self.TriggerBoxLocation`) false false)
  (`SceneComponent.SetRelativeScale3D` _triggerbox (`self.TriggerBoxSize`)))